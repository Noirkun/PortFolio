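; BP_SavePoint is a save point actor that opens a save menu when the player presses interact inside its trigger box.
; BeginPlay creates the prompt and save menu widgets, then binds SaveMenuEvent to the push event on BP_ThirdPersonCharacter.
; Box overlaps show or hide the prompt and set InBox without filtering the overlapping actor.
; When InBox is true, SaveMenuEvent swaps the prompt for the menu.
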(event `self.ReceiveBeginPlay`
  (bind _returnvalue (`|CreateWidget` "/Game/Widget/WBP_PressInteract.WBP_PressInteract_C"))
  (set `self.PressWidget` _returnvalue)
  (bind _returnvalue_2 (`|CreateWidget` "/Game/Widget/WBP_SavePoints.WBP_SavePoints_C"))
  (add `/Game/ThirdPerson/Blueprints/BP_ThirdPersonCharacter.PushEvent` (cast `/Game/ThirdPerson/Blueprints/BP_ThirdPersonCharacter` (`GameplayStatics.GetPlayerPawn` 0) :!pure true) (delegate `SaveMenuEvent`)))

(event `SaveMenuEvent`
  (if (`self.bInBox`)
    (`UserWidget.AddToViewport` (stale `self.ReceiveBeginPlay` _returnvalue_2) 0)
    (`Widget.RemoveFromParent` (`self.PressWidget`))))

(event `self.Box.OnComponentBeginOverlap`
  (params (OverlappedComponent :type "PrimitiveComponent Object Reference") (OtherActor :type "Actor Object Reference") (OtherComp :type "PrimitiveComponent Object Reference") (OtherBodyIndex :type Integer) (bFromSweep :type Boolean) (SweepResult :type "HitResult Structure (by ref)"))
  (`UserWidget.AddToViewport` (`self.PressWidget`) 0)
  (set `self.bInBox` true))

(event `self.Box.OnComponentEndOverlap`
  (params (OverlappedComponent :type "PrimitiveComponent Object Reference") (OtherActor :type "Actor Object Reference") (OtherComp :type "PrimitiveComponent Object Reference") (OtherBodyIndex :type Integer))
  (`Widget.RemoveFromParent` (`self.PressWidget`))
  (set `self.bInBox` false))

(fn `UserConstructionScript`)